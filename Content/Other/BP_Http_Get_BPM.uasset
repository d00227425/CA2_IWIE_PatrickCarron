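; Actor that fetches a BPM value from an Adafruit IO feed and plays a beat sound at a matching tempo.
; A Delay on Tick throttles HTTP GETs to roughly every 15 seconds, using a hard-coded API key in the URL.
; Success parses the JSON last value into BPM and enters an endless Delay loop playing double beats.
; The loop's period is the BPM interval plus a fixed half-second gap.
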(event EventBeginPlay)

(event Collision|EventActorBeginOverlap
  (params (OtherActor :type Actor%20Object%20Reference)))

(event EventTick
  (params (DeltaSeconds :type Float%20%28single-precision%29))
  (Utilities|FlowControl|Delay 15.0)
  (bind _result_body (|HttpRequest "https://io.adafruit.com/api/v2/D00227425/feeds/bpm?x-aio-key=aio_FhzD27N65aQEaat8J6MTM6DONYSU" "Get")
    (:On%20Success
      (bind _outjsonobject (Class|JsonBlueprintFunctionLibrary|FromString _result_body))
      (bind _outvalue (|GetJsonField _outjsonobject "last_value"))
      (Development|PrintString (Utilities|String|ToString(Integer) _outvalue) true true "(R=0.000000,G=0.660000,B=1.000000,A=1.000000)" 4.0)
      (Variables|Default|SetBPM (Math|Conversions|ToFloat(Integer) _outvalue))
      (Utilities|FlowControl|Delay (/ 1.0 (/ (Variables|Default|GetBPM) 6e+01)) :!label _label)
      (Audio|PlaySound2D "/Game/Other/beatcue.beatcue" 1.0 1.0 0.0 0 0)
      (Utilities|FlowControl|Delay 0.5)
      (Audio|PlaySound2D "/Game/Other/beatcue.beatcue" 1.0 1.0 0.0 0 0)
      (goto _label))))

(fn ConstructionScript)